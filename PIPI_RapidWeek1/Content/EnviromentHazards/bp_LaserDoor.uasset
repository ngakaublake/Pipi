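; Laser door environment hazard Blueprint, apparently unfinished, meant to flicker and switch laser modes.
; BeginPlay loops over Cube2's children, adding to LaserArray with no connected item and calling LaserFlicker1, then prints the count.
; LaserFlicker1 deactivates each entry's root component after a short delay, with no reactivation.
; The "Laser" tag filter is disconnected, LaserDoor is uncalled here, and LaserMode1 is empty.
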(event `self.ReceiveBeginPlay`
  (for _array_element (`SceneComponent.GetChildrenComponents` (`self.Cube2`) false)
    (`KismetArrayLibrary.Array_Add` (`self.LaserArray`))
    (`self.Laser Flicker 1`))
  (`KismetSystemLibrary.PrintString` (`KismetStringLibrary.Conv_IntToString` (`KismetArrayLibrary.Array_Length` (`self.LaserArray`)))))

(event `Laser Flicker 1`
  (`KismetSystemLibrary.Delay` 0.2)
  (for _array_element (`self.LaserArray`)
    (`ActorComponent.SetActive` (`Actor.RootComponent` _array_element) false false)))

(fn `Laser Mode 1`)

(fn `LaserDoor`
  (if (== (`self.CurrentMode`) 0)
    (`self.Laser Mode 1`)))

(fn `UserConstructionScript`)