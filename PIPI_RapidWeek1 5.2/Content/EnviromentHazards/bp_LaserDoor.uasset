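; Laser door environmental hazard that drives seven child bp_Laser actors in a repeating staggered sequence.
; BeginPlay gathers the lasers into an array and starts LaserFlicker1, which pauses, calls SetLaserActive on each in turn with a short delay, then restarts itself.
; The LaserDoor mode selector is never called here and leads only to an empty LaserMode1; a component-search alternative is left disconnected.
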(event `self.ReceiveBeginPlay`
  (set `self.LaserArray` (`|MakeArray` (`ChildActorComponent.ChildActor` (`self.Laser1`)) (`ChildActorComponent.ChildActor` (`self.Laser2`)) (`ChildActorComponent.ChildActor` (`self.Laser3`)) (`ChildActorComponent.ChildActor` (`self.Laser4`)) (`ChildActorComponent.ChildActor` (`self.Laser5`)) (`ChildActorComponent.ChildActor` (`self.Laser6`)) (`ChildActorComponent.ChildActor` (`self.Laser7`))))
  (set `self.MaxLaserNum` (- (`KismetArrayLibrary.Array_Length` (`self.LaserArray`)) 1))
  (`self.Laser Flicker 1`))

(event `Laser Flicker 1`
  (set `self.CurrentLaser` 0)
  (`KismetSystemLibrary.Delay` 3.0)
  (bind _asbp_laser (cast `/Game/EnviromentHazards/bp_Laser` (`|GetArrayItem` (`self.LaserArray`) (`self.CurrentLaser`)) :!label _label))
  (`/Game/EnviromentHazards/bp_Laser.SetLaserActive` _asbp_laser)
  (`KismetSystemLibrary.Delay` 0.15)
  (if (== (`self.MaxLaserNum`) (`self.CurrentLaser`))
    (`self.Laser Flicker 1`)
    (else
      (bind _result (`/Engine/EditorBlueprintResources/StandardMacros.IncrementInt` (`self.CurrentLaser`))
        (:`  `
          (set `self.CurrentLaser` _result)
          (goto _label))))))

(fn `Laser Mode 1`)

(fn `LaserDoor`
  (if (== (`self.CurrentMode`) 0)
    (`self.Laser Mode 1`)))

(fn `UserConstructionScript`)