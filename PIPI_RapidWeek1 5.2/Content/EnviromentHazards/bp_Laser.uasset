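; Laser hazard actor that destroys the player's BP_ThirdPersonCharacter when it overlaps the laser while active.
; Begin and end overlap track the player, and Tick checks that state against IsActive, so switching on over a player also kills.
; SetLaserActive toggles IsActive rather than setting it, and actor visibility follows the flag from BeginPlay onward.
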(event `self.ReceiveBeginPlay`
  (`self.SetActorHiddenInGame` (not (`self.IsActive`))))

(event `self.ReceiveActorBeginOverlap`
  (params (OtherActor :type "Actor Object Reference"))
  (bind _asbp_third_person_character (cast `/Game/ThirdPerson/Blueprints/BP_ThirdPersonCharacter` OtherActor))
  (set `self.IsplayerOverlapping` true)
  (set `self.As BP Third Person Character` _asbp_third_person_character))

(event `self.ReceiveActorEndOverlap`
  (params (OtherActor :type "Actor Object Reference"))
  (cast `/Game/ThirdPerson/Blueprints/BP_ThirdPersonCharacter` OtherActor)
  (set `self.IsplayerOverlapping` false))

(event `self.ReceiveTick`
  (params (DeltaSeconds :type "Float (single-precision)"))
  (if (`self.IsplayerOverlapping`)
    (if (`self.IsActive`)
      (`self.K2_DestroyActor` (`self.As BP Third Person Character`)))))

(fn `SetLaserActive`
  (bind _output_get (set `self.IsActive` (not (`self.IsActive`))))
  (`self.SetActorHiddenInGame` (not _output_get)))

(fn `UserConstructionScript`)