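; Door button hazard actor that opens a matching pair of sliding door panels when the third-person character overlaps it.
; On overlap it prints a debug string and calls Interact, which searches all left and right panel actors for a DoorTag equal to its ButtonTag.
; Each matching left and right pair is told to open.
; A velocity-threshold DestroyActor branch is present but never runs.
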(event `self.ReceiveActorBeginOverlap`
  (params (OtherActor :type "Actor Object Reference"))
  (`KismetSystemLibrary.PrintString` "Hello")
  (cast `/Game/ThirdPerson/Blueprints/BP_ThirdPersonCharacter` OtherActor)
  (`/Game/EnviromentHazards/bp_InteractInterface.Interact`))

(event `/Game/EnviromentHazards/bp_InteractInterface.Interact`
  (bind _outactors (`GameplayStatics.GetAllActorsOfClass` "/Game/EnviromentHazards/bp_DoorPanelLeft.bp_DoorPanelLeft_C"))
  (for _array_element _outactors
    (if (== (`/Game/EnviromentHazards/bp_DoorPanelLeft.DoorTag` _array_element) (`self.ButtonTag`))
      (bind _outactors_2 (`GameplayStatics.GetAllActorsOfClass` "/Game/EnviromentHazards/bp_DoorPanelRight.bp_DoorPanelRight_C"))
      (for _array_element_2 _outactors_2
        (if (== (`/Game/EnviromentHazards/bp_DoorPanelRight.DoorTag` _array_element_2) (`self.ButtonTag`))
          (`/Game/EnviromentHazards/bp_DoorPanelLeft.OpenDoorLeft` _array_element)
          (`/Game/EnviromentHazards/bp_DoorPanelRight.OpenDoorRight` _array_element_2))))))

(fn `UserConstructionScript`)