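; A destructible water flask hazard that breaks when moving fast enough, awarding score and leaving a puddle.
; BeginPlay overrides the static mesh's mass, then Tick compares its velocity to a required threshold while the flask is unbroken.
; Breaking adds score through the default game mode, spawns a small puddle at the flask's location and scale, then destroys the actor.
; An older delayed-destroy physics break path remains unconnected.
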(event `self.ReceiveBeginPlay`
  (`parent.ReceiveBeginPlay`)
  (`PrimitiveComponent.SetMassOverrideInKg` (`self.StaticMesh`) "None" (`self.Mass`) true))

(event `self.ReceiveActorBeginOverlap`
  (params (OtherActor :type "Actor Object Reference"))
  (`parent.ReceiveActorBeginOverlap` OtherActor))

(event `self.ReceiveTick`
  (params (DeltaSeconds :type "Float (single-precision)"))
  (`parent.ReceiveTick` DeltaSeconds)
  (if (`self.isBroken`)
    (if (== 0.0 (`KismetMathLibrary.VSize` (`SceneComponent.GetComponentVelocity` (`self.StaticMesh`))))
      _)
    (elif (>= (`KismetMathLibrary.VSize` (`SceneComponent.GetComponentVelocity` (`self.StaticMesh`))) (`self.VelocityRequired`))
      (`self.ManageBreak`))))

(event `ManageBreak`
  (bind (_returnvalue_location _returnvalue_rotation _returnvalue_scale) (`KismetMathLibrary.BreakTransform` (`self.GetTransform`)))
  (set `self.isBroken` true)
  (bind _asbp_default_game_mode (cast `/Game/CoreGame/bp_DefaultGameMode` (`GameplayStatics.GetGameMode`)))
  (`/Game/CoreGame/bp_DefaultGameMode.AddScore` _asbp_default_game_mode (`self.Score`))
  (`|SpawnActorFromClass` "/Game/EnviromentHazards/bp_PuddleSmall.bp_PuddleSmall_C" (`KismetMathLibrary.MakeTransform` _returnvalue_location (struct) _returnvalue_scale) "AdjustIfPossibleButAlwaysSpawn" "MultiplyWithRoot" null null)
  (`self.K2_DestroyActor`))

(fn `UserConstructionScript`
  (`parent.UserConstructionScript`))