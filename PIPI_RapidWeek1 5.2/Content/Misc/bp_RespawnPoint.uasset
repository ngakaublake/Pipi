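; Respawn point actor that becomes the active checkpoint when the third-person character overlaps it.
; On overlap it finds every respawn point in the level, marks only itself active and calls ManageSpawn on each.
; ManageSpawn turns the point light green on the active point and red on the others.
; The active point also writes its transform to the game mode as the respawn transform.
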(event `self.ReceiveActorBeginOverlap`
  (params (OtherActor :type "Actor Object Reference"))
  (cast `/Game/ThirdPerson/Blueprints/BP_ThirdPersonCharacter` OtherActor)
  (bind _outactors (`GameplayStatics.GetAllActorsOfClass` "bp_RespawnPoint_C"))
  (for _array_element _outactors
    (if (!= _array_element self)
      (set `/Game/Misc/bp_RespawnPoint.isActiveSpawn` false _array_element)
      (else
        (set `/Game/Misc/bp_RespawnPoint.isActiveSpawn` true _array_element)))
    (`self.ManageSpawn` _array_element)))

(event `ManageSpawn`
  (bind _pointlight (`self.PointLight`))
  (if (`self.isActiveSpawn`)
    (`LightComponent.SetLightColor` _pointlight (struct :`R` 0.014323 :`G` 1.0 :`A` 1.0) true)
    (bind _asbp_default_game_mode (cast `/Game/CoreGame/bp_DefaultGameMode` (`GameplayStatics.GetGameMode`)))
    (set `/Game/CoreGame/bp_DefaultGameMode.RespawnTrans` (`self.GetTransform`) _asbp_default_game_mode)
    (else
      (`LightComponent.SetLightColor` _pointlight (struct :`R` 1.0 :`G` 0.070089 :`A` 1.0) true))))

(fn `UserConstructionScript`)