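; Default game mode that handles pausing, player respawning and score tracking.
; On BeginPlay it enables input for the first player controller, so pressing P opens the pause menu widget, switches to UI-only input with a visible cursor and pauses the game.
; RespawnPlayer spawns a new actor of the given character's class at a stored respawn transform and possesses it.
; AddScore accumulates points and prints the total on screen.
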(event `self.ReceiveBeginPlay`
  (`self.EnableInput` (`GameplayStatics.GetPlayerController` 0)))

(event `Key|P`
  (params (Key :type "Key Structure"))
  (bind _returnvalue (`GameplayStatics.GetPlayerController` 0))
  (:`Pressed`
    (bind _returnvalue_2 (`|CreateWidget` "/Game/HUD/wbp_PauseMenu.wbp_PauseMenu_C"))
    (`UserWidget.AddToViewport` _returnvalue_2 0)
    (`WidgetBlueprintLibrary.SetInputMode_UIOnlyEx` _returnvalue _returnvalue_2)
    (set `PlayerController.bShowMouseCursor` true _returnvalue)
    (`GameplayStatics.SetGamePaused` true)))

(fn `AddScore`
  (params (ScoreToAdd :type Integer))
  (bind _output_get (set `self.Score` (+ (`self.Score`) ScoreToAdd)))
  (`KismetSystemLibrary.PrintString` (`KismetStringLibrary.Conv_IntToString` _output_get) true true (struct :`R` 1.0 :`G` 0.085798 :`A` 1.0)))

(fn `RespawnPlayer`
  (params (CharacterClass :type "Character Object Reference"))
  (bind _returnvalue (`|SpawnActorFromClass` (`GameplayStatics.GetObjectClass` CharacterClass) (`self.RespawnTrans`) "Undefined" "MultiplyWithRoot" null null))
  (`Controller.Possess` (`GameplayStatics.GetPlayerController` 0) _returnvalue)
  (`KismetSystemLibrary.PrintString` "RESPAWN OVER"))

(fn `UserConstructionScript`)