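; Game state Blueprint that keeps a game clock as minute and second counters.
; BeginPlay sets a non-looping timer on GameTIMER, using the current server world time as its delay, and stores the handle.
; GameTIMER increments Secs, rolls over into Mins after 59, then calls itself directly with no delay or exit condition, so the count is not paced to real seconds.
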(event `self.ReceiveBeginPlay`
  (bind _returnvalue (`KismetSystemLibrary.K2_SetTimerDelegate` (delegate `GameTIMER`) (`self.GetServerWorldTimeSeconds`)))
  (set `self.GameClockTimerHandle` _returnvalue))

(event `GameTIMER`
  (bind _secs (`self.Secs`))
  (if (!= _secs 59)
    (bind _result (`/Engine/EditorBlueprintResources/StandardMacros.IncrementInt` _secs)
      (:`  `
        (set `self.Secs` _result)))
    (else
      (bind _result_2 (`/Engine/EditorBlueprintResources/StandardMacros.IncrementInt` (`self.Mins`))
        (:`  `
          (set `self.Mins` _result_2)
          (set `self.Secs` 0)))))
  (`self.GameTIMER`))

(fn `UserConstructionScript`)