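; BP_WorldPercentBar is an in-world progress bar showing the score as a fraction of the required score.
; Every Tick it reads Score and ScoreRequired from bp_DefaultGameMode and caps the ratio at 1.
; Bar's Y scale follows that ratio while Base's takes the remainder.
; Bar is offset and rotated 180 degrees relative to its parent, and both transforms are rewritten each frame.
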(event `self.ReceiveTick`
  (params (DeltaSeconds :type "Float (single-precision)"))
  (bind _asbp_default_game_mode (cast `/Game/CoreGame/bp_DefaultGameMode` (`GameplayStatics.GetGameMode`)))
  (bind _output_get (set `self.Percentage` (/ (`/Game/CoreGame/bp_DefaultGameMode.Score` _asbp_default_game_mode) (`/Game/CoreGame/bp_DefaultGameMode.ScoreRequired` _asbp_default_game_mode))))
  (if (not (<= _output_get 1.0))
    (set `self.Percentage` 1.0))
  (`SceneComponent.K2_SetRelativeTransform` (`self.Bar`) (`KismetMathLibrary.MakeTransform` (50.0 100.0 0.0) (struct :`Yaw` 180.0) (`KismetMathLibrary.MakeVector` 0.5 (`self.Percentage`) 0.5)) false false)
  (`SceneComponent.K2_SetRelativeTransform` (`self.Base`) (`KismetMathLibrary.MakeTransform` (0.0 0.0 0.0) (struct) (`KismetMathLibrary.MakeVector` 0.5 (- 1.0 (`self.Percentage`)) 0.5)) false false))

(fn `UserConstructionScript`)