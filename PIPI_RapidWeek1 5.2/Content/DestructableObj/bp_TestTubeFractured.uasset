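; Fractured test tube actor that carries a Geometry Collection for a destructible debris effect.
; Its ManageSpawn event takes a mass and a force, overrides the collection's mass, applies the force as an impulse and prints the force magnitude.
; The event only proceeds if the player character is a BP_ThirdPersonCharacter, and the actor destroys itself after a short delay.
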(event `ManageSpawn`
  (params (Mass :type "Float (double-precision)") (Force :type "Vector Structure"))
  (bind _asbp_third_person_character (cast `/Game/ThirdPerson/Blueprints/BP_ThirdPersonCharacter` (`GameplayStatics.GetPlayerCharacter` 0)))
  (`PrimitiveComponent.SetMassOverrideInKg` (`self.GeometryCollection`) "None" Mass true)
  (`PrimitiveComponent.AddImpulse` (`self.GeometryCollection`) Force "None" false)
  (`KismetSystemLibrary.PrintString` (`KismetStringLibrary.Conv_DoubleToString` (`KismetMathLibrary.VSize` Force)))
  (`KismetSystemLibrary.Delay` 5.0)
  (`self.K2_DestroyActor`))

(fn `UserConstructionScript`)