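; Destructible bowl actor built on a Chaos Geometry Collection that awards score to bp_DefaultGameMode when it breaks.
; BeginPlay applies the Mass override, and the first Chaos break event triggers ManageBreak, guarded by IsBroken.
; ManageBreak adds Score, plays the Impact effect at the break location, then destroys the actor after a short delay.
; Unconnected leftover nodes hold alternative velocity-threshold and fractured-flask spawn logic.
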(event `self.ReceiveBeginPlay`
  (`parent.ReceiveBeginPlay`)
  (`PrimitiveComponent.SetMassOverrideInKg` (`self.GeometryCollection`) "None" (`self.Mass`) true))

(event `self.ReceiveActorBeginOverlap`
  (params (OtherActor :type "Actor Object Reference"))
  (`parent.ReceiveActorBeginOverlap` OtherActor))

(event `self.ReceiveTick`
  (params (DeltaSeconds :type "Float (single-precision)"))
  (`parent.ReceiveTick` DeltaSeconds))

(event `self.GeometryCollection.OnChaosBreakEvent`
  (params (BreakEvent :type "ChaosBreakEvent Structure (by ref)"))
  (set `self.Break Event Location` BreakEvent_Location)
  (if (not (`self.isBroken`))
    (`self.ManageBreak`)))

(event `ManageBreak`
  (set `self.isBroken` true)
  (bind _asbp_default_game_mode (cast `/Game/CoreGame/bp_DefaultGameMode` (`GameplayStatics.GetGameMode`)))
  (`/Game/CoreGame/bp_DefaultGameMode.AddScore` _asbp_default_game_mode (`self.Score`))
  (`SceneComponent.K2_SetWorldTransform` (`self.Impact`) (`KismetMathLibrary.Conv_VectorToTransform` (`self.Break Event Location`)) false true)
  (`ActorComponent.Activate` (`self.Impact`) true)
  (`KismetSystemLibrary.Delay` 5.0)
  (`self.K2_DestroyActor`))

(fn `UserConstructionScript`
  (`parent.UserConstructionScript`))