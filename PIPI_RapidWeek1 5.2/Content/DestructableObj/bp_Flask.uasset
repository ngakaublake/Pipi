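; bp_Flask is a destructible flask that awards score when it moves fast enough to count as broken.
; BeginPlay overrides the static mesh's mass, and Tick compares its velocity with a required threshold until it breaks.
; ManageBreak sets the broken flag, adds the score through bp_DefaultGameMode, then destroys the actor after a short delay.
; An unconnected duplicate of that break logic, which also toggles physics simulation, never runs.
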(event `self.ReceiveBeginPlay`
  (`parent.ReceiveBeginPlay`)
  (`PrimitiveComponent.SetMassOverrideInKg` (`self.StaticMesh`) "None" (`self.Mass`) true))

(event `self.ReceiveActorBeginOverlap`
  (params (OtherActor :type "Actor Object Reference"))
  (`parent.ReceiveActorBeginOverlap` OtherActor))

(event `self.ReceiveTick`
  (params (DeltaSeconds :type "Float (single-precision)"))
  (`parent.ReceiveTick` DeltaSeconds)
  (if (`self.isBroken`)
    _
    (elif (>= (`KismetMathLibrary.VSize` (`SceneComponent.GetComponentVelocity` (`self.StaticMesh`))) (`self.VelocityRequired`))
      (`self.ManageBreak`))))

(event `ManageBreak`
  (set `self.isBroken` true)
  (bind _asbp_default_game_mode (cast `/Game/CoreGame/bp_DefaultGameMode` (`GameplayStatics.GetGameMode`)))
  (`/Game/CoreGame/bp_DefaultGameMode.AddScore` _asbp_default_game_mode (`self.Score`))
  (`KismetSystemLibrary.Delay` 3.0)
  (`self.K2_DestroyActor`))

(fn `UserConstructionScript`
  (`parent.UserConstructionScript`))