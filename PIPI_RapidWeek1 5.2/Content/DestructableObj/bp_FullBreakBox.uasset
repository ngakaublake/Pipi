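; Destructible box actor that reacts when its Chaos Geometry Collection breaks.
; The first break event stores its location and sets a broken flag, so later breaks do not retrigger the response.
; It then moves the Impact component to that location and activates it.
; After a short delay it destroys the Geometry Collection component to clear the debris, without destroying the actor itself.
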(event `self.GeometryCollection.OnChaosBreakEvent`
  (params (BreakEvent :type "ChaosBreakEvent Structure (by ref)"))
  (set `self.Break Event Location` BreakEvent_Location)
  (if (not (`self.IsBroken`))
    (`self.ManageBreak`)))

(event `ManageBreak`
  (bind _impact (`self.Impact`))
  (set `self.isBroken` true)
  (`SceneComponent.K2_SetWorldTransform` _impact (`KismetMathLibrary.Conv_VectorToTransform` (`self.Break Event Location`)) false true)
  (`ActorComponent.Activate` _impact true)
  (`KismetSystemLibrary.Delay` 5.0)
  (`ActorComponent.K2_DestroyComponent` (`self.GeometryCollection`)))

(fn `UserConstructionScript`)