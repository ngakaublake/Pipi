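; Fractured flask debris actor that represents a broken flask as a physics-driven Geometry Collection.
; Its ManageSpawn event takes a mass and force, overrides the collection's mass, and applies the force scaled up as an impulse to throw the pieces.
; After a short delay the actor destroys itself, so the debris is temporary.
; Unconnected material and AddForce nodes remain in the graph and never run.
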(event `ManageSpawn`
  (params (Mass :type "Float (double-precision)") (Force :type "Vector Structure"))
  (`PrimitiveComponent.SetMassOverrideInKg` (`self.GeometryCollection`) "None" Mass true)
  (`PrimitiveComponent.AddImpulse` (`self.GeometryCollection`) (* Force (3.0 3.0 3.0)) "None" false)
  (`KismetSystemLibrary.Delay` 5.0)
  (`self.K2_DestroyActor`))

(fn `UserConstructionScript`)